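; BP_SPawnableObject is a touch-reactive actor that flies toward the player's camera when tapped.
; On BeginPlay it spawns another instance of its own class at Location, so each new copy also spawns one.
; A touch plays the MoveTowardsCamera timeline, lerping the actor from Location to the camera position.
; A one-second Delay on the timeline update then destroys the spawned child, not the touched actor.
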(event `self.ReceiveBeginPlay`
  (bind _returnvalue (`|SpawnActorFromClass` "BP_SPawnableObject_C" (`KismetMathLibrary.MakeTransform` (`self.Location`) (struct :`Pitch` 10.0 :`Yaw` 10.0 :`Roll` 10.0)) "Undefined" "MultiplyWithRoot" null null)))

(event `self.ReceiveActorOnInputTouchBegin`
  (params (FingerIndex :type "ETouchIndex Enum" :default "Touch1"))
  (bind (_direction _alpha) (`Timeline|MoveTowardsCamera`)
    (:`Update`
      (`self.K2_SetActorLocation` (`KismetMathLibrary.VLerp` (`self.Location`) (`PlayerCameraManager.GetCameraLocation` (`GameplayStatics.GetPlayerCameraManager` 0)) _alpha))
      (`KismetSystemLibrary.Delay` 1.0)
      (`self.K2_DestroyActor` (stale `self.ReceiveBeginPlay` _returnvalue)))))

(fn `UserConstructionScript`)